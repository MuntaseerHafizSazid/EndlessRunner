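; Endless-runner track tile that randomly populates itself on BeginPlay with obstacles, rows of cash and powerups at lane markers.
; When the player overlaps its Box, it asks MainGameMode to spawn the next tile, then destroys itself after a short delay.
; If the game mode's Change flag is set, it instead spawns several tiles, repositions the player and clears the flag.
; A long timeout also destroys the tile.
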(event `self.ReceiveBeginPlay`
  (`self.Spawn Obstacle`)
  (`self.Spawn Cash`)
  (`self.Spawn Powerups`)
  (`KismetSystemLibrary.Delay` 180.0)
  (`self.K2_DestroyActor`))

(event `self.Box.OnComponentBeginOverlap`
  (params (OverlappedComponent :type "PrimitiveComponent Object Reference") (OtherActor :type "Actor Object Reference") (OtherComp :type "PrimitiveComponent Object Reference") (OtherBodyIndex :type Integer) (bFromSweep :type Boolean) (SweepResult :type "HitResult Structure (by ref)"))
  (bind _returnvalue (`GameplayStatics.GetPlayerCharacter` 0))
  (bind _returnvalue_x (`KismetMathLibrary.BreakVector` (`SceneComponent.K2_GetComponentLocation` (`Character.CapsuleComponent` _returnvalue))))
  ;[1 1 1] Auto Tile Generation and self-destruction
  (cast `/Game/Blueprints/MainGameCharacter_BP` OtherActor)
  (bind _asmain_game_mode (cast `/Game/Blueprints/MainGameMode` (`GameplayStatics.GetGameMode`)))
  (if (`/Game/Blueprints/MainGameMode.Change` _asmain_game_mode)
    (for _ (range 3)
      (`/Game/Blueprints/MainGameMode.SpawnTile` _asmain_game_mode))
    (`self.K2_SetActorLocation` _returnvalue (`KismetMathLibrary.MakeVector` _returnvalue_x -2800.0 10.0) false false)
    (`KismetSystemLibrary.Delay` 0.45)
    (set `/Game/Blueprints/MainGameMode.Change` false _asmain_game_mode)
    (`self.K2_DestroyActor`)
    (else
      (`KismetSystemLibrary.Delay` 0.45)
      (`/Game/Blueprints/MainGameMode.SpawnTile` _asmain_game_mode)
      (`self.K2_DestroyActor`))))

(fn `Spawn Cash`
  (bind _nextcashspawntransform_location (`KismetMathLibrary.BreakTransform` (`self.NextCashSpawnTransform`)))
  (bind _nextcashspawntransform_location_2 (`KismetMathLibrary.BreakTransform` (`self.NextCashSpawnTransform`)))
  (bind _nextcashspawntransform_location_3 (`KismetMathLibrary.BreakTransform` (`self.NextCashSpawnTransform`)))
  (bind _nextcashspawntransform_location_4 (`KismetMathLibrary.BreakTransform` (`self.NextCashSpawnTransform`)))
  (bind _nextcashspawntransform_location_5 (`KismetMathLibrary.BreakTransform` (`self.NextCashSpawnTransform`)))
  (bind _nextcashspawntransform_location_6 (`KismetMathLibrary.BreakTransform` (`self.NextCashSpawnTransform`)))
  (switch `int` (`KismetMathLibrary.RandomIntegerInRange` 0 2)
    (:`0`
      (set `self.NextCashSpawnTransform` (`SceneComponent.K2_GetComponentToWorld` (`self.LaneC1`)))
      (for _ (range 6)
        (`|SpawnActorFromClass` "/Game/Blueprints/Cash.Cash_C" (`self.NextCashSpawnTransform`) "Undefined" "OverrideRootScale" null null)
        (set `self.NextCashSpawnTransform` (`KismetMathLibrary.MakeTransform` (+ _nextcashspawntransform_location_5 (0.0 50.0 0.0)))))
      (set `self.NextCashSpawnTransform` (`SceneComponent.K2_GetComponentToWorld` (`self.LaneC2`)))
      (for _ (range 6)
        (`|SpawnActorFromClass` "/Game/Blueprints/Cash.Cash_C" (`self.NextCashSpawnTransform`) "Undefined" "OverrideRootScale" null null)
        (set `self.NextCashSpawnTransform` (`KismetMathLibrary.MakeTransform` (+ _nextcashspawntransform_location_6 (0.0 50.0 0.0))))))
    (:`1`
      (set `self.NextCashSpawnTransform` (`SceneComponent.K2_GetComponentToWorld` (`self.LaneC2`)))
      (for _ (range 6)
        (`|SpawnActorFromClass` "/Game/Blueprints/Cash.Cash_C" (`self.NextCashSpawnTransform`) "Undefined" "OverrideRootScale" null null)
        (set `self.NextCashSpawnTransform` (`KismetMathLibrary.MakeTransform` (+ _nextcashspawntransform_location_2 (0.0 50.0 0.0)))))
      (set `self.NextCashSpawnTransform` (`SceneComponent.K2_GetComponentToWorld` (`self.LaneC3`)))
      (for _ (range 6)
        (`|SpawnActorFromClass` "/Game/Blueprints/Cash.Cash_C" (`self.NextCashSpawnTransform`) "Undefined" "OverrideRootScale" null null)
        (set `self.NextCashSpawnTransform` (`KismetMathLibrary.MakeTransform` (+ _nextcashspawntransform_location_3 (0.0 50.0 0.0))))))
    (:`2`
      (set `self.NextCashSpawnTransform` (`SceneComponent.K2_GetComponentToWorld` (`self.LaneC1`)))
      (for _ (range 6)
        (`|SpawnActorFromClass` "/Game/Blueprints/Cash.Cash_C" (`self.NextCashSpawnTransform`) "Undefined" "OverrideRootScale" null null)
        (set `self.NextCashSpawnTransform` (`KismetMathLibrary.MakeTransform` (+ _nextcashspawntransform_location_4 (0.0 50.0 0.0)))))
      (set `self.NextCashSpawnTransform` (`SceneComponent.K2_GetComponentToWorld` (`self.LaneC3`)))
      (for _ (range 6)
        (`|SpawnActorFromClass` "/Game/Blueprints/Cash.Cash_C" (`self.NextCashSpawnTransform`) "Undefined" "OverrideRootScale" null null)
        (set `self.NextCashSpawnTransform` (`KismetMathLibrary.MakeTransform` (+ _nextcashspawntransform_location (0.0 50.0 0.0))))))))

(fn `Spawn Obstacle`
  (bind _returnvalue (`SceneComponent.K2_GetComponentToWorld` (`self.Lane1`)))
  (bind _returnvalue_2 (`SceneComponent.K2_GetComponentToWorld` (`self.Lane5`)))
  (bind _returnvalue_3 (`SceneComponent.K2_GetComponentToWorld` (`self.Lane6`)))
  (bind _returnvalue_4 (`SceneComponent.K2_GetComponentToWorld` (`self.Lane7`)))
  (bind _returnvalue_5 (`SceneComponent.K2_GetComponentToWorld` (`self.Lane8`)))
  (bind _returnvalue_6 (`SceneComponent.K2_GetComponentToWorld` (`self.Lane9`)))
  (bind _returnvalue_7 (`SceneComponent.K2_GetComponentToWorld` (`self.Lane2`)))
  (bind _returnvalue_8 (`SceneComponent.K2_GetComponentToWorld` (`self.Lane10`)))
  (bind _returnvalue_9 (`SceneComponent.K2_GetComponentToWorld` (`self.Lane3`)))
  (bind _returnvalue_10 (`SceneComponent.K2_GetComponentToWorld` (`self.Lane4`)))
  (switch `int` (`KismetMathLibrary.RandomIntegerInRange` 0 5)
    (:`Default`
      _)
    (:`0`
      (`|SpawnActorFromClass` "/Game/Blueprints/ObstacleGround.ObstacleGround_C" _returnvalue "Undefined" "OverrideRootScale" null null))
    (:`1`
      (`|SpawnActorFromClass` "/Game/Blueprints/ObstacleBox.ObstacleBox_C" _returnvalue "Undefined" "OverrideRootScale" null null))
    (:`2`
      (`|SpawnActorFromClass` "/Game/Blueprints/ObstacleBigBox.ObstacleBigBox_C" _returnvalue "Undefined" "OverrideRootScale" null null))
    (:`3`
      (`|SpawnActorFromClass` "/Game/Blueprints/ObstacleCutter.ObstacleCutter_C" _returnvalue "Undefined" "OverrideRootScale" null null)))
  (switch `int` (`KismetMathLibrary.RandomIntegerInRange` 0 5)
    (:`Default`
      _)
    (:`0`
      (`|SpawnActorFromClass` "/Game/Blueprints/ObstacleGround.ObstacleGround_C" _returnvalue_7 "Undefined" "OverrideRootScale" null null))
    (:`1`
      (`|SpawnActorFromClass` "/Game/Blueprints/ObstacleBox.ObstacleBox_C" _returnvalue_7 "Undefined" "OverrideRootScale" null null))
    (:`2`
      (`|SpawnActorFromClass` "/Game/Blueprints/ObstacleBigBox.ObstacleBigBox_C" _returnvalue_7 "Undefined" "OverrideRootScale" null null))
    (:`3`
      (`|SpawnActorFromClass` "/Game/Blueprints/ObstacleCutter.ObstacleCutter_C" _returnvalue_7 "Undefined" "OverrideRootScale" null null)))
  (switch `int` (`KismetMathLibrary.RandomIntegerInRange` 0 5)
    (:`Default`
      _)
    (:`0`
      (`|SpawnActorFromClass` "/Game/Blueprints/ObstacleGround.ObstacleGround_C" _returnvalue_9 "Undefined" "OverrideRootScale" null null))
    (:`1`
      (`|SpawnActorFromClass` "/Game/Blueprints/ObstacleBox.ObstacleBox_C" _returnvalue_9 "Undefined" "OverrideRootScale" null null))
    (:`2`
      (`|SpawnActorFromClass` "/Game/Blueprints/ObstacleBigBox.ObstacleBigBox_C" _returnvalue_9 "Undefined" "OverrideRootScale" null null))
    (:`3`
      (`|SpawnActorFromClass` "/Game/Blueprints/ObstacleCutter.ObstacleCutter_C" _returnvalue_9 "Undefined" "OverrideRootScale" null null)))
  (switch `int` (`KismetMathLibrary.RandomIntegerInRange` 0 5)
    (:`Default`
      _)
    (:`0`
      (`|SpawnActorFromClass` "/Game/Blueprints/ObstacleGround.ObstacleGround_C" _returnvalue_10 "Undefined" "OverrideRootScale" null null))
    (:`1`
      (`|SpawnActorFromClass` "/Game/Blueprints/ObstacleBox.ObstacleBox_C" _returnvalue_10 "Undefined" "OverrideRootScale" null null))
    (:`2`
      (`|SpawnActorFromClass` "/Game/Blueprints/ObstacleBigBox.ObstacleBigBox_C" _returnvalue_10 "Undefined" "OverrideRootScale" null null))
    (:`3`
      (`|SpawnActorFromClass` "/Game/Blueprints/ObstacleCutter.ObstacleCutter_C" _returnvalue_10 "Undefined" "OverrideRootScale" null null)))
  (switch `int` (`KismetMathLibrary.RandomIntegerInRange` 0 5)
    (:`Default`
      _)
    (:`0`
      (`|SpawnActorFromClass` "/Game/Blueprints/ObstacleGround.ObstacleGround_C" _returnvalue_2 "Undefined" "OverrideRootScale" null null))
    (:`1`
      (`|SpawnActorFromClass` "/Game/Blueprints/ObstacleBox.ObstacleBox_C" _returnvalue_2 "Undefined" "OverrideRootScale" null null))
    (:`2`
      (`|SpawnActorFromClass` "/Game/Blueprints/ObstacleBigBox.ObstacleBigBox_C" _returnvalue_2 "Undefined" "OverrideRootScale" null null))
    (:`3`
      (`|SpawnActorFromClass` "/Game/Blueprints/ObstacleCutter.ObstacleCutter_C" _returnvalue_2 "Undefined" "OverrideRootScale" null null)))
  (switch `int` (`KismetMathLibrary.RandomIntegerInRange` 0 5)
    (:`Default`
      _)
    (:`0`
      (`|SpawnActorFromClass` "/Game/Blueprints/ObstacleGround.ObstacleGround_C" _returnvalue_3 "Undefined" "OverrideRootScale" null null))
    (:`1`
      (`|SpawnActorFromClass` "/Game/Blueprints/ObstacleBox.ObstacleBox_C" _returnvalue_3 "Undefined" "OverrideRootScale" null null))
    (:`2`
      (`|SpawnActorFromClass` "/Game/Blueprints/ObstacleBigBox.ObstacleBigBox_C" _returnvalue_3 "Undefined" "OverrideRootScale" null null))
    (:`3`
      (`|SpawnActorFromClass` "/Game/Blueprints/ObstacleCutter.ObstacleCutter_C" _returnvalue_3 "Undefined" "OverrideRootScale" null null)))
  (switch `int` (`KismetMathLibrary.RandomIntegerInRange` 0 5)
    (:`Default`
      _)
    (:`0`
      (`|SpawnActorFromClass` "/Game/Blueprints/ObstacleGround.ObstacleGround_C" _returnvalue_4 "Undefined" "OverrideRootScale" null null))
    (:`1`
      (`|SpawnActorFromClass` "/Game/Blueprints/ObstacleBox.ObstacleBox_C" _returnvalue_4 "Undefined" "OverrideRootScale" null null))
    (:`2`
      (`|SpawnActorFromClass` "/Game/Blueprints/ObstacleBigBox.ObstacleBigBox_C" _returnvalue_4 "Undefined" "OverrideRootScale" null null))
    (:`3`
      (`|SpawnActorFromClass` "/Game/Blueprints/ObstacleCutter.ObstacleCutter_C" _returnvalue_4 "Undefined" "OverrideRootScale" null null)))
  (switch `int` (`KismetMathLibrary.RandomIntegerInRange` 0 5)
    (:`Default`
      _)
    (:`0`
      (`|SpawnActorFromClass` "/Game/Blueprints/ObstacleGround.ObstacleGround_C" _returnvalue_5 "Undefined" "OverrideRootScale" null null))
    (:`1`
      (`|SpawnActorFromClass` "/Game/Blueprints/ObstacleBox.ObstacleBox_C" _returnvalue_5 "Undefined" "OverrideRootScale" null null))
    (:`2`
      (`|SpawnActorFromClass` "/Game/Blueprints/ObstacleBigBox.ObstacleBigBox_C" _returnvalue_5 "Undefined" "OverrideRootScale" null null))
    (:`3`
      (`|SpawnActorFromClass` "/Game/Blueprints/ObstacleCutter.ObstacleCutter_C" _returnvalue_5 "Undefined" "OverrideRootScale" null null)))
  (switch `int` (`KismetMathLibrary.RandomIntegerInRange` 0 5)
    (:`Default`
      _)
    (:`0`
      (`|SpawnActorFromClass` "/Game/Blueprints/ObstacleGround.ObstacleGround_C" _returnvalue_6 "Undefined" "OverrideRootScale" null null))
    (:`1`
      (`|SpawnActorFromClass` "/Game/Blueprints/ObstacleBox.ObstacleBox_C" _returnvalue_6 "Undefined" "OverrideRootScale" null null))
    (:`2`
      (`|SpawnActorFromClass` "/Game/Blueprints/ObstacleBigBox.ObstacleBigBox_C" _returnvalue_6 "Undefined" "OverrideRootScale" null null))
    (:`3`
      (`|SpawnActorFromClass` "/Game/Blueprints/ObstacleCutter.ObstacleCutter_C" _returnvalue_6 "Undefined" "OverrideRootScale" null null)))
  (switch `int` (`KismetMathLibrary.RandomIntegerInRange` 0 5)
    (:`0`
      (`|SpawnActorFromClass` "/Game/Blueprints/ObstacleGround.ObstacleGround_C" _returnvalue_8 "Undefined" "OverrideRootScale" null null))
    (:`1`
      (`|SpawnActorFromClass` "/Game/Blueprints/ObstacleBox.ObstacleBox_C" _returnvalue_8 "Undefined" "OverrideRootScale" null null))
    (:`2`
      (`|SpawnActorFromClass` "/Game/Blueprints/ObstacleBigBox.ObstacleBigBox_C" _returnvalue_8 "Undefined" "OverrideRootScale" null null))
    (:`3`
      (`|SpawnActorFromClass` "/Game/Blueprints/ObstacleCutter.ObstacleCutter_C" _returnvalue_8 "Undefined" "OverrideRootScale" null null))))

(fn `Spawn Powerups`
  (bind _returnvalue (`SceneComponent.K2_GetComponentToWorld` (`self.LaneP1`)))
  (bind _returnvalue_2 (`SceneComponent.K2_GetComponentToWorld` (`self.LaneP2`)))
  (switch `int` (`KismetMathLibrary.RandomIntegerInRange` 0 4)
    (:`Default`
      _)
    (:`0`
      (`|SpawnActorFromClass` "/Game/Blueprints/ScoreMultiplier.ScoreMultiplier_C" _returnvalue "Undefined" "OverrideRootScale" null null))
    (:`1`
      (`|SpawnActorFromClass` "/Game/Blueprints/SpeedIncreaser.SpeedIncreaser_C" _returnvalue "Undefined" "OverrideRootScale" null null))
    (:`2`
      (`|SpawnActorFromClass` "/Game/Blueprints/SpeedDecreaser.SpeedDecreaser_C" _returnvalue "Undefined" "OverrideRootScale" null null))
    (:`3`
      (`|SpawnActorFromClass` "/Game/Blueprints/Magnet.Magnet_C" _returnvalue "Undefined" "OverrideRootScale" null null)))
  (switch `int` (`KismetMathLibrary.RandomIntegerInRange` 0 4)
    (:`0`
      (`|SpawnActorFromClass` "/Game/Blueprints/ScoreMultiplier.ScoreMultiplier_C" _returnvalue_2 "Undefined" "OverrideRootScale" null null))
    (:`1`
      (`|SpawnActorFromClass` "/Game/Blueprints/SpeedIncreaser.SpeedIncreaser_C" _returnvalue_2 "Undefined" "OverrideRootScale" null null))
    (:`2`
      (`|SpawnActorFromClass` "/Game/Blueprints/SpeedDecreaser.SpeedDecreaser_C" _returnvalue_2 "Undefined" "OverrideRootScale" null null))
    (:`3`
      (`|SpawnActorFromClass` "/Game/Blueprints/Magnet.Magnet_C" _returnvalue_2 "Undefined" "OverrideRootScale" null null))))

(fn `UserConstructionScript`)