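; Game mode that lays out a randomized track of tiles when play begins.
; BeginPlay loops to call SpawnTile, also creating and adding a PlayerUI widget on every iteration, so the widgets stack.
; SpawnTile picks one of six tile classes at random, spawns it at SpawnPoint, then advances that point by a fixed negative Y offset.
; An unconnected leftover branch instead derives the next point from the spawned tile's own SpawnPoint component.
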(event `self.ReceiveBeginPlay`
  (for _ (range 6)
    (`self.SpawnTile`)
    (bind _returnvalue (`|CreateWidget` "/Game/UI/PlayerUI.PlayerUI_C"))
    (`UserWidget.AddToViewport` _returnvalue 0)))

(fn `SpawnTile`
  (bind _spawnpoint (`self.SpawnPoint`))
  (bind _spawnpoint_location (`KismetMathLibrary.BreakTransform` (`self.SpawnPoint`)))
  (bind _spawnpoint_location_2 (`KismetMathLibrary.BreakTransform` (`self.SpawnPoint`)))
  (bind _spawnpoint_location_3 (`KismetMathLibrary.BreakTransform` (`self.SpawnPoint`)))
  (bind _spawnpoint_location_4 (`KismetMathLibrary.BreakTransform` (`self.SpawnPoint`)))
  (bind _spawnpoint_location_5 (`KismetMathLibrary.BreakTransform` (`self.SpawnPoint`)))
  (bind _spawnpoint_location_6 (`KismetMathLibrary.BreakTransform` (`self.SpawnPoint`)))
  (switch `int` (`KismetMathLibrary.RandomIntegerInRange` 0 5)
    (:`0`
      (`|SpawnActorFromClass` "/Game/Blueprints/Tile001.Tile001_C" _spawnpoint "Undefined" "OverrideRootScale" null null)
      (set `self.SpawnPoint` (`KismetMathLibrary.MakeTransform` (+ _spawnpoint_location_6 (0.0 -6000.0 0.0)))))
    (:`1`
      (`|SpawnActorFromClass` "/Game/Blueprints/Tile002.Tile002_C" _spawnpoint "Undefined" "OverrideRootScale" null null)
      (set `self.SpawnPoint` (`KismetMathLibrary.MakeTransform` (+ _spawnpoint_location (0.0 -6000.0 0.0)))))
    (:`2`
      (`|SpawnActorFromClass` "/Game/Blueprints/Tile003.Tile003_C" _spawnpoint "Undefined" "OverrideRootScale" null null)
      (set `self.SpawnPoint` (`KismetMathLibrary.MakeTransform` (+ _spawnpoint_location_2 (0.0 -6000.0 0.0)))))
    (:`3`
      (`|SpawnActorFromClass` "/Game/Blueprints/Tile004.Tile004_C" _spawnpoint "Undefined" "OverrideRootScale" null null)
      (set `self.SpawnPoint` (`KismetMathLibrary.MakeTransform` (+ _spawnpoint_location_3 (0.0 -6000.0 0.0)))))
    (:`4`
      (`|SpawnActorFromClass` "/Game/Blueprints/Tile005.Tile005_C" _spawnpoint "Undefined" "OverrideRootScale" null null)
      (set `self.SpawnPoint` (`KismetMathLibrary.MakeTransform` (+ _spawnpoint_location_4 (0.0 -6000.0 0.0)))))
    (:`5`
      (`|SpawnActorFromClass` "/Game/Blueprints/Tile006.Tile006_C" _spawnpoint "Undefined" "OverrideRootScale" null null)
      (set `self.SpawnPoint` (`KismetMathLibrary.MakeTransform` (+ _spawnpoint_location_5 (0.0 -6000.0 0.0)))))))

(fn `UserConstructionScript`)