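; Cash pickup actor that adds money to the player's total when the main character walks into it.
; On overlap with MainGameCharacter_BP, it adds a fixed 20 to CurrentCash on MainGameMode, plays a cash register beep and destroys itself.
; Uncollected pickups remove themselves after a seven-minute delay started at BeginPlay.
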(event `self.ReceiveBeginPlay`
  (`KismetSystemLibrary.Delay` 420.0)
  (`self.K2_DestroyActor`))

(event `self.ReceiveActorBeginOverlap`
  (params (OtherActor :type "Actor Object Reference"))
  (cast `/Game/Blueprints/MainGameCharacter_BP` OtherActor)
  (bind _asmain_game_mode (cast `/Game/Blueprints/MainGameMode` (`GameplayStatics.GetGameMode`)))
  (set `/Game/Blueprints/MainGameMode.CurrentCash` (+ (`/Game/Blueprints/MainGameMode.CurrentCash` _asmain_game_mode) 20) _asmain_game_mode)
  (`GameplayStatics.PlaySound2D` "/Game/Sounds/ES_Cash_Register_Beep_-_SFX_Producer.ES_Cash_Register_Beep_-_SFX_Producer" 1.0 1.0 0.0 null null)
  (`self.K2_DestroyActor`))

(fn `UserConstructionScript`)