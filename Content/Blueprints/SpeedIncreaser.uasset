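; SpeedIncreaser is a pickup actor that permanently speeds up the main game character on overlap.
; It adds a fixed bonus to walk speed, then derives crouched speed from the raised walk speed plus the same bonus, so crouching ends up faster than walking.
; It plays a 2D sound and destroys itself on pickup, or self-destructs seven minutes after BeginPlay if uncollected.
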(event `self.ReceiveBeginPlay`
  (`KismetSystemLibrary.Delay` 420.0)
  (`self.K2_DestroyActor`))

(event `self.ReceiveActorBeginOverlap`
  (params (OtherActor :type "Actor Object Reference"))
  (bind _asmain_game_character_bp (cast `/Game/Blueprints/MainGameCharacter_BP` OtherActor))
  (bind _charactermovement (`Character.CharacterMovement` _asmain_game_character_bp))
  (bind _returnvalue (+ (`CharacterMovementComponent.MaxWalkSpeed` _charactermovement) 200.0))
  (set `CharacterMovementComponent.MaxWalkSpeed` _returnvalue _charactermovement)
  (set `CharacterMovementComponent.MaxWalkSpeedCrouched` _returnvalue _charactermovement)
  (`GameplayStatics.PlaySound2D` "/Game/Sounds/message-incoming-132126.message-incoming-132126" 1.0 1.0 0.0 null null)
  (`self.K2_DestroyActor`))

(fn `UserConstructionScript`)