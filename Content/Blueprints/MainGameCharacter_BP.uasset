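; Player character for an endless runner on a skateboard, running forward automatically with rising speed.
; Tick drives movement and eases the camera through crouches, while a delayed step keeps increasing walk speeds.
; Input lerps between five lanes on a shared timeline, jumps with chained skateboard timelines, crouches, or pauses into the Quit widget.
; DeathFunction destroys the board, ragdolls the mesh, stops movement and saves the GameMode score if it matches or beats the high score.
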(event `InputAction|Quit`
  (params (Key :type "Key Structure"))
  ;[1 1 1] Quit
  (:`Pressed`
    (bind _returnvalue (`|CreateWidget` "/Game/UI/Quit.Quit_C"))
    (`UserWidget.AddToViewport` _returnvalue 0)
    (set `PlayerController.bShowMouseCursor` true (`GameplayStatics.GetPlayerController` 0))
    (`GameplayStatics.SetGamePaused` true)))

(event `self.ReceiveTick`
  (params (DeltaSeconds :type "Float (single-precision)"))
  ;[1 1 1] Movement and Crouch
  (`self.AddMovementInput` (`KismetMathLibrary.GetForwardVector` (`KismetMathLibrary.MakeRotator` 0.0 0.0 (.yaw (`self.GetControlRotation`)))))
  (bind _output_get (set `self.CurrentInterpolatedLocation` (`KismetMathLibrary.VInterpTo` (`self.CurrentInterpolatedLocation`) (`self.BaseCameraLocation`) DeltaSeconds 10.0)))
  (`SceneComponent.K2_SetRelativeLocation` (`self.FollowCamera`) _output_get false false)
  (`KismetSystemLibrary.Delay` 1.0)
  (bind _asmain_game_character_bp (cast `/Game/Blueprints/MainGameCharacter_BP` (`GameplayStatics.GetPlayerCharacter` 0)))
  (bind _charactermovement (`Character.CharacterMovement` _asmain_game_character_bp))
  (bind _returnvalue (+ (`CharacterMovementComponent.MaxWalkSpeed` _charactermovement) 10.0))
  (set `CharacterMovementComponent.MaxWalkSpeed` _returnvalue _charactermovement)
  (set `CharacterMovementComponent.MaxWalkSpeedCrouched` _returnvalue _charactermovement))

(event `InputAction|Jump`
  (params (Key :type "Key Structure"))
  (bind _skateboard (`self.SkateBoard`))
  (bind _skateboard_2 (`self.SkateBoard`))
  (bind (_returnvalue_x _returnvalue_y _returnvalue_z) (`KismetMathLibrary.BreakVector` (`SceneComponent.K2_GetComponentLocation` _skateboard_2)))
  (bind (_returnvalue_x_2 _returnvalue_y_2 _returnvalue_z_2) (`KismetMathLibrary.BreakVector` (`SceneComponent.K2_GetComponentLocation` _skateboard)))
  ;[1 1 1] Jump Function
  (:`Pressed`
    (if (not (`NavMovementComponent.IsCrouching` (`self.CharacterMovement`)))
      (`self.Jump`)
      (bind (_direction _newtrack_0) (`Timeline|Timeline_0` :!via `PlayFromStart`)
        (:`Update`
          (`SceneComponent.K2_SetWorldLocation` _skateboard_2 (`KismetMathLibrary.MakeVector` _returnvalue_x _returnvalue_y (+ _newtrack_0 _returnvalue_z)) false false))
        (:`Finished`
          (bind (_direction_2 _newtrack_0_2) (`Timeline|Timeline_1` :!via `PlayFromStart`)
            (:`Update`
              (`SceneComponent.K2_SetWorldLocation` _skateboard (`KismetMathLibrary.MakeVector` _returnvalue_x_2 _returnvalue_y_2 (+ _newtrack_0_2 _returnvalue_z_2)) false false))))))))

(event `self.ReceiveBeginPlay`
  ;[1 1 1] Movement and Crouch
  (bind _output_get (set `self.BaseCameraLocation` (`SceneComponent.RelativeLocation` (`self.FollowCamera`))))
  (set `self.CurrentInterpolatedLocation` _output_get))

(event `self.K2_OnStartCrouch`
  (params (HalfHeightAdjust :type "Float (single-precision)") (ScaledHalfHeightAdjust :type "Float (single-precision)"))
  ;[1 1 1] Movement and Crouch
  (if (not (`NavMovementComponent.IsFalling` (`self.CharacterMovement`)))
    (set `self.CurrentInterpolatedLocation` (+ (`self.BaseCameraLocation`) (`KismetMathLibrary.MakeVector` 0.0 0.0 ScaledHalfHeightAdjust)))))

(event `InputAction|LeftSwitch`
  (params (Key :type "Key Structure"))
  (bind _lanex (`self.LaneX`))
  (bind (_returnvalue_x _returnvalue_y _returnvalue_z) (`KismetMathLibrary.BreakVector` (`SceneComponent.K2_GetComponentLocation` (`self.CapsuleComponent`))))
  ;[1 1 1] Left and Right Switching
  (:`Pressed`
    (set `self.NewLane` (`KismetMathLibrary.Clamp` (+ (`self.Lane`) 1) 0 4))
    (if (not (`self.isLooping`))
      (bind (_direction _lane_x) (`Timeline|Lerp Timeline` :!via `PlayFromStart` :!label _label)
        (:`Update`
          (set `self.isLooping` true)
          (`self.K2_SetActorLocation` (`KismetMathLibrary.MakeVector` (`KismetMathLibrary.Lerp` (`|GetArrayItem` _lanex (`self.Lane`)) (`|GetArrayItem` _lanex (`self.NewLane`)) _lane_x) _returnvalue_y _returnvalue_z)))
        (:`Finished`
          (set `self.Lane` (`self.NewLane`))
          (set `self.isLooping` false))))))

(event `self.K2_OnEndCrouch`
  (params (HalfHeightAdjust :type "Float (single-precision)") (ScaledHalfHeightAdjust :type "Float (single-precision)"))
  ;[1 1 1] Movement and Crouch
  (if (not (`NavMovementComponent.IsFalling` (`self.CharacterMovement`)))
    (set `self.CurrentInterpolatedLocation` (- (`self.BaseCameraLocation`) (`KismetMathLibrary.MakeVector` 0.0 0.0 ScaledHalfHeightAdjust)))))

(event `InputAction|Crouch`
  (params (Key :type "Key Structure"))
  ;[1 1 1] Movement and Crouch
  (:`Pressed`
    (`self.Crouch`))
  (:`Released`
    (`self.UnCrouch`)))

(event `InputAction|RightSwitch`
  (params (Key :type "Key Structure"))
  ;[1 1 1] Left and Right Switching
  (:`Pressed`
    (set `self.NewLane` (`KismetMathLibrary.Clamp` (+ (`self.Lane`) -1) 0 4))
    (if (not (`self.isLooping`))
      (goto _label :!via `PlayFromStart`))))

(fn `DeathFunction`
  (set `self.Death` true)
  (`ActorComponent.K2_DestroyComponent` (`self.SkateBoard`))
  (`PrimitiveComponent.SetSimulatePhysics` (`self.Mesh`) true)
  (`CharacterMovementComponent.DisableMovement` (`self.CharacterMovement`))
  (bind _asmain_game_mode (cast `/Game/Blueprints/MainGameMode` (`GameplayStatics.GetGameMode`)))
  (bind _returnvalue (`GameplayStatics.DoesSaveGameExist` "HighScoreData"))
  (if _returnvalue
    (bind _returnvalue_2 (`GameplayStatics.LoadGameFromSlot` "HighScoreData"))
    (bind _output_get (set `self.SaverSubClass` _returnvalue_2))
    (bind _aseternal_runner_save_game (cast `/Game/Blueprints/EternalRunnerSaveGame` _output_get))
    (bind _currentscore (`/Game/Blueprints/MainGameMode.CurrentScore` _asmain_game_mode))
    (if (>= _currentscore (`/Game/Blueprints/EternalRunnerSaveGame.HighScoreValue` _aseternal_runner_save_game))
      (set `/Game/Blueprints/EternalRunnerSaveGame.HighScoreValue` _currentscore _aseternal_runner_save_game)
      (`GameplayStatics.SaveGameToSlot` (`self.SaverSubClass`) "HighScoreData"))
    (else
      (bind _returnvalue_3 (`GameplayStatics.CreateSaveGameObject` "/Game/Blueprints/EternalRunnerSaveGame.EternalRunnerSaveGame_C"))
      (bind _output_get_2 (set `self.SaverSubClass` _returnvalue_3))
      (bind _aseternal_runner_save_game_2 (cast `/Game/Blueprints/EternalRunnerSaveGame` _output_get_2))
      (set `/Game/Blueprints/EternalRunnerSaveGame.HighScoreValue` _currentscore _aseternal_runner_save_game_2)
      (`GameplayStatics.SaveGameToSlot` (`self.SaverSubClass`) "HighScoreData"))))

(fn `UserConstructionScript`)