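; Self-replacing track tile, apparently for an endless runner, that fills itself with random obstacles and cash.
; On BeginPlay, each of ten lane markers independently rolls for one of four obstacle types or none.
; A coin flip decides whether two rows of Cash spawn, stepped along world Y from two markers.
; When the player character leaves the Box, it waits briefly, asks MainGameMode for another tile and destroys itself.
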(event `self.ReceiveBeginPlay`
  (`self.SpawnObstacle`)
  (`self.Spawn Cash`))

(event `self.box.OnComponentEndOverlap`
  (params (OverlappedComponent :type "PrimitiveComponent Object Reference") (OtherActor :type "Actor Object Reference") (OtherComp :type "PrimitiveComponent Object Reference") (OtherBodyIndex :type Integer))
  ;[1 1 1] Auto Tile Genaration and Self Destruction
  (cast `/Game/Blueprints/MainGameCharacter_BP` OtherActor)
  (bind _asmain_game_mode (cast `/Game/Blueprints/MainGameMode` (`GameplayStatics.GetGameMode`)))
  (`KismetSystemLibrary.Delay` 0.45)
  (`/Game/Blueprints/MainGameMode.SpawnTile` _asmain_game_mode)
  (`self.K2_DestroyActor`))

(fn `Spawn Cash`
  (bind _nextcashspawntransform_location (`KismetMathLibrary.BreakTransform` (`self.NextCashSpawnTransform`)))
  (bind _nextcashspawntransform_location_2 (`KismetMathLibrary.BreakTransform` (`self.NextCashSpawnTransform`)))
  (switch `int` (`KismetMathLibrary.RandomIntegerInRange` 0 1)
    (:`0`
      (set `self.NextCashSpawnTransform` (`SceneComponent.K2_GetComponentToWorld` (`self.LaneC1`)))
      (for _ (range 6)
        (`|SpawnActorFromClass` "/Game/Blueprints/Cash.Cash_C" (`self.NextCashSpawnTransform`) "Undefined" "OverrideRootScale" null null)
        (set `self.NextCashSpawnTransform` (`KismetMathLibrary.MakeTransform` (+ _nextcashspawntransform_location (0.0 50.0 0.0)))))
      (set `self.NextCashSpawnTransform` (`SceneComponent.K2_GetComponentToWorld` (`self.LaneC2`)))
      (for _ (range 6)
        (`|SpawnActorFromClass` "/Game/Blueprints/Cash.Cash_C" (`self.NextCashSpawnTransform`) "Undefined" "OverrideRootScale" null null)
        (set `self.NextCashSpawnTransform` (`KismetMathLibrary.MakeTransform` (+ _nextcashspawntransform_location_2 (0.0 50.0 0.0))))))))

(fn `SpawnObstacle`
  (bind _returnvalue (`SceneComponent.K2_GetComponentToWorld` (`self.Lane1`)))
  (bind _returnvalue_2 (`SceneComponent.K2_GetComponentToWorld` (`self.Lane5`)))
  (bind _returnvalue_3 (`SceneComponent.K2_GetComponentToWorld` (`self.Lane6`)))
  (bind _returnvalue_4 (`SceneComponent.K2_GetComponentToWorld` (`self.Lane7`)))
  (bind _returnvalue_5 (`SceneComponent.K2_GetComponentToWorld` (`self.Lane8`)))
  (bind _returnvalue_6 (`SceneComponent.K2_GetComponentToWorld` (`self.Lane9`)))
  (bind _returnvalue_7 (`SceneComponent.K2_GetComponentToWorld` (`self.Lane2`)))
  (bind _returnvalue_8 (`SceneComponent.K2_GetComponentToWorld` (`self.Lane10`)))
  (bind _returnvalue_9 (`SceneComponent.K2_GetComponentToWorld` (`self.Lane3`)))
  (bind _returnvalue_10 (`SceneComponent.K2_GetComponentToWorld` (`self.Lane4`)))
  (switch `int` (`KismetMathLibrary.RandomIntegerInRange` 0 5)
    (:`Default`
      _)
    (:`0`
      (`|SpawnActorFromClass` "/Game/Blueprints/ObstacleGround.ObstacleGround_C" _returnvalue "Undefined" "OverrideRootScale" null null))
    (:`1`
      (`|SpawnActorFromClass` "/Game/Blueprints/ObstacleBox.ObstacleBox_C" _returnvalue "Undefined" "OverrideRootScale" null null))
    (:`2`
      (`|SpawnActorFromClass` "/Game/Blueprints/ObstacleBigBox.ObstacleBigBox_C" _returnvalue "Undefined" "OverrideRootScale" null null))
    (:`3`
      (`|SpawnActorFromClass` "/Game/Blueprints/ObstacleCutter.ObstacleCutter_C" _returnvalue "Undefined" "OverrideRootScale" null null)))
  (switch `int` (`KismetMathLibrary.RandomIntegerInRange` 0 5)
    (:`Default`
      _)
    (:`0`
      (`|SpawnActorFromClass` "/Game/Blueprints/ObstacleGround.ObstacleGround_C" _returnvalue_7 "Undefined" "OverrideRootScale" null null))
    (:`1`
      (`|SpawnActorFromClass` "/Game/Blueprints/ObstacleBox.ObstacleBox_C" _returnvalue_7 "Undefined" "OverrideRootScale" null null))
    (:`2`
      (`|SpawnActorFromClass` "/Game/Blueprints/ObstacleBigBox.ObstacleBigBox_C" _returnvalue_7 "Undefined" "OverrideRootScale" null null))
    (:`3`
      (`|SpawnActorFromClass` "/Game/Blueprints/ObstacleCutter.ObstacleCutter_C" _returnvalue_7 "Undefined" "OverrideRootScale" null null)))
  (switch `int` (`KismetMathLibrary.RandomIntegerInRange` 0 5)
    (:`Default`
      _)
    (:`0`
      (`|SpawnActorFromClass` "/Game/Blueprints/ObstacleGround.ObstacleGround_C" _returnvalue_9 "Undefined" "OverrideRootScale" null null))
    (:`1`
      (`|SpawnActorFromClass` "/Game/Blueprints/ObstacleBox.ObstacleBox_C" _returnvalue_9 "Undefined" "OverrideRootScale" null null))
    (:`2`
      (`|SpawnActorFromClass` "/Game/Blueprints/ObstacleBigBox.ObstacleBigBox_C" _returnvalue_9 "Undefined" "OverrideRootScale" null null))
    (:`3`
      (`|SpawnActorFromClass` "/Game/Blueprints/ObstacleCutter.ObstacleCutter_C" _returnvalue_9 "Undefined" "OverrideRootScale" null null)))
  (switch `int` (`KismetMathLibrary.RandomIntegerInRange` 0 5)
    (:`Default`
      _)
    (:`0`
      (`|SpawnActorFromClass` "/Game/Blueprints/ObstacleGround.ObstacleGround_C" _returnvalue_10 "Undefined" "OverrideRootScale" null null))
    (:`1`
      (`|SpawnActorFromClass` "/Game/Blueprints/ObstacleBox.ObstacleBox_C" _returnvalue_10 "Undefined" "OverrideRootScale" null null))
    (:`2`
      (`|SpawnActorFromClass` "/Game/Blueprints/ObstacleBigBox.ObstacleBigBox_C" _returnvalue_10 "Undefined" "OverrideRootScale" null null))
    (:`3`
      (`|SpawnActorFromClass` "/Game/Blueprints/ObstacleCutter.ObstacleCutter_C" _returnvalue_10 "Undefined" "OverrideRootScale" null null)))
  (switch `int` (`KismetMathLibrary.RandomIntegerInRange` 0 5)
    (:`Default`
      _)
    (:`0`
      (`|SpawnActorFromClass` "/Game/Blueprints/ObstacleGround.ObstacleGround_C" _returnvalue_2 "Undefined" "OverrideRootScale" null null))
    (:`1`
      (`|SpawnActorFromClass` "/Game/Blueprints/ObstacleBox.ObstacleBox_C" _returnvalue_2 "Undefined" "OverrideRootScale" null null))
    (:`2`
      (`|SpawnActorFromClass` "/Game/Blueprints/ObstacleBigBox.ObstacleBigBox_C" _returnvalue_2 "Undefined" "OverrideRootScale" null null))
    (:`3`
      (`|SpawnActorFromClass` "/Game/Blueprints/ObstacleCutter.ObstacleCutter_C" _returnvalue_2 "Undefined" "OverrideRootScale" null null)))
  (switch `int` (`KismetMathLibrary.RandomIntegerInRange` 0 5)
    (:`Default`
      _)
    (:`0`
      (`|SpawnActorFromClass` "/Game/Blueprints/ObstacleGround.ObstacleGround_C" _returnvalue_3 "Undefined" "OverrideRootScale" null null))
    (:`1`
      (`|SpawnActorFromClass` "/Game/Blueprints/ObstacleBox.ObstacleBox_C" _returnvalue_3 "Undefined" "OverrideRootScale" null null))
    (:`2`
      (`|SpawnActorFromClass` "/Game/Blueprints/ObstacleBigBox.ObstacleBigBox_C" _returnvalue_3 "Undefined" "OverrideRootScale" null null))
    (:`3`
      (`|SpawnActorFromClass` "/Game/Blueprints/ObstacleCutter.ObstacleCutter_C" _returnvalue_3 "Undefined" "OverrideRootScale" null null)))
  (switch `int` (`KismetMathLibrary.RandomIntegerInRange` 0 5)
    (:`Default`
      _)
    (:`0`
      (`|SpawnActorFromClass` "/Game/Blueprints/ObstacleGround.ObstacleGround_C" _returnvalue_4 "Undefined" "OverrideRootScale" null null))
    (:`1`
      (`|SpawnActorFromClass` "/Game/Blueprints/ObstacleBox.ObstacleBox_C" _returnvalue_4 "Undefined" "OverrideRootScale" null null))
    (:`2`
      (`|SpawnActorFromClass` "/Game/Blueprints/ObstacleBigBox.ObstacleBigBox_C" _returnvalue_4 "Undefined" "OverrideRootScale" null null))
    (:`3`
      (`|SpawnActorFromClass` "/Game/Blueprints/ObstacleCutter.ObstacleCutter_C" _returnvalue_4 "Undefined" "OverrideRootScale" null null)))
  (switch `int` (`KismetMathLibrary.RandomIntegerInRange` 0 5)
    (:`Default`
      _)
    (:`0`
      (`|SpawnActorFromClass` "/Game/Blueprints/ObstacleGround.ObstacleGround_C" _returnvalue_5 "Undefined" "OverrideRootScale" null null))
    (:`1`
      (`|SpawnActorFromClass` "/Game/Blueprints/ObstacleBox.ObstacleBox_C" _returnvalue_5 "Undefined" "OverrideRootScale" null null))
    (:`2`
      (`|SpawnActorFromClass` "/Game/Blueprints/ObstacleBigBox.ObstacleBigBox_C" _returnvalue_5 "Undefined" "OverrideRootScale" null null))
    (:`3`
      (`|SpawnActorFromClass` "/Game/Blueprints/ObstacleCutter.ObstacleCutter_C" _returnvalue_5 "Undefined" "OverrideRootScale" null null)))
  (switch `int` (`KismetMathLibrary.RandomIntegerInRange` 0 5)
    (:`Default`
      _)
    (:`0`
      (`|SpawnActorFromClass` "/Game/Blueprints/ObstacleGround.ObstacleGround_C" _returnvalue_6 "Undefined" "OverrideRootScale" null null))
    (:`1`
      (`|SpawnActorFromClass` "/Game/Blueprints/ObstacleBox.ObstacleBox_C" _returnvalue_6 "Undefined" "OverrideRootScale" null null))
    (:`2`
      (`|SpawnActorFromClass` "/Game/Blueprints/ObstacleBigBox.ObstacleBigBox_C" _returnvalue_6 "Undefined" "OverrideRootScale" null null))
    (:`3`
      (`|SpawnActorFromClass` "/Game/Blueprints/ObstacleCutter.ObstacleCutter_C" _returnvalue_6 "Undefined" "OverrideRootScale" null null)))
  (switch `int` (`KismetMathLibrary.RandomIntegerInRange` 0 5)
    (:`0`
      (`|SpawnActorFromClass` "/Game/Blueprints/ObstacleGround.ObstacleGround_C" _returnvalue_8 "Undefined" "OverrideRootScale" null null))
    (:`1`
      (`|SpawnActorFromClass` "/Game/Blueprints/ObstacleBox.ObstacleBox_C" _returnvalue_8 "Undefined" "OverrideRootScale" null null))
    (:`2`
      (`|SpawnActorFromClass` "/Game/Blueprints/ObstacleBigBox.ObstacleBigBox_C" _returnvalue_8 "Undefined" "OverrideRootScale" null null))
    (:`3`
      (`|SpawnActorFromClass` "/Game/Blueprints/ObstacleCutter.ObstacleCutter_C" _returnvalue_8 "Undefined" "OverrideRootScale" null null))))

(fn `UserConstructionScript`)