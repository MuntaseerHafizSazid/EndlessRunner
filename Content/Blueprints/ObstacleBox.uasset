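; ObstacleBox is an obstacle actor that ends the game when the player character touches it.
; Its box overlap calls DeathFunction on MainGameCharacter_BP, waits briefly, then removes the MainGameMode widget, shows an EndGame widget with the mouse cursor and pauses the game.
; Each instance also destroys itself on a fixed timer started at BeginPlay.
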(event `self.ReceiveBeginPlay`
  (`KismetSystemLibrary.Delay` 180.0)
  (`self.K2_DestroyActor`))

(event `self.ObstacleBox.OnComponentBeginOverlap`
  (params (OverlappedComponent :type "PrimitiveComponent Object Reference") (OtherActor :type "Actor Object Reference") (OtherComp :type "PrimitiveComponent Object Reference") (OtherBodyIndex :type Integer) (bFromSweep :type Boolean) (SweepResult :type "HitResult Structure (by ref)"))
  (bind _asmain_game_character_bp (cast `/Game/Blueprints/MainGameCharacter_BP` OtherActor))
  (`/Game/Blueprints/MainGameCharacter_BP.DeathFunction` _asmain_game_character_bp)
  (`KismetSystemLibrary.Delay` 3.0)
  (bind _asmain_game_mode (cast `/Game/Blueprints/MainGameMode` (`GameplayStatics.GetGameMode`)))
  (`Widget.RemoveFromParent` (`/Game/Blueprints/MainGameMode.Widget` _asmain_game_mode))
  (bind _returnvalue (`|CreateWidget` "/Game/UI/EndGame.EndGame_C"))
  (`UserWidget.AddToViewport` _returnvalue 0)
  (set `PlayerController.bShowMouseCursor` true (`GameplayStatics.GetPlayerController` 0))
  (`GameplayStatics.SetGamePaused` true))

(fn `UserConstructionScript`)